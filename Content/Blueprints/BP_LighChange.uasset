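; Race signal light actor that runs a start light sequence and plays a crowd reaction when its trigger is crossed.
; On BeginPlay the pole material switches from red to green after a short delay, then the trigger's collision is disabled for a longer delay before overlap detection is bound.
; An overlap by the NPC car's AI trigger plays a losing crowd sound, any other plays a cheer, then the handler attempts to unbind.
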(event Custom|collision%20check
  (params (OverlappedComponent :type Primitive%20Component%20Object%20Reference) (OtherActor :type Actor%20Object%20Reference) (OtherComp :type Primitive%20Component%20Object%20Reference) (OtherBodyIndex :type Integer) (bFromSweep :type Boolean) (SweepResult :type Hit%20Result%20Structure%20%28by%20ref%29))
  (if (== OtherComp (Variables|/Game/VehicleTemplate/Blueprints/SportsCar/BP_NPC_Car.BP_NPC_Car_C|GetAItrigger (Variables|Default|GetNPCCar)))
    (Audio|PlaySound2D "/Game/Sounds/NewAudio/Crowd_Loose.Crowd_Loose" 1.0 1.0 0.0 0 0)
    (else
      (Audio|PlaySound2D "/Game/Sounds/chereSound.chereSound" 1.0 1.0 0.0 0 0)))
  (Collision|UnbindEventfromOnComponentBeginOverlap (Variables|Default|GetTrigger) (EventDispatchers|CreateEvent :!event Custom|collision%20check)))

(event EventBeginPlay
  (Rendering|Material|SetMaterial (Variables|Default|GetLight_Pole) 1 "/Game/Assets/Tex/Signal_1_Signal_Light_Tex_BaseColor_Mat_Red.Signal_1_Signal_Light_Tex_BaseColor_Mat_Red")
  (Utilities|FlowControl|Delay 3.0)
  (Rendering|Material|SetMaterial (Variables|Default|GetLight_Pole) 1 "/Game/Assets/Tex/Signal_1_Signal_Light_Tex_BaseColor_Mat_Green.Signal_1_Signal_Light_Tex_BaseColor_Mat_Green")
  (Collision|SetCollisionEnabled (Variables|Default|GetTrigger) "NoCollision")
  (Utilities|FlowControl|Delay 1e+01)
  (Collision|SetCollisionEnabled (Variables|Default|GetTrigger) "QueryOnly")
  (Collision|BindEventtoOnComponentBeginOverlap (Variables|Default|GetTrigger) (EventDispatchers|CreateEvent :!event Custom|collision%20check)))

(event Collision|EventActorBeginOverlap
  (params (OtherActor :type Actor%20Object%20Reference)))

(event EventTick
  (params (DeltaSeconds :type Float%20%28single-precision%29)))

(fn ConstructionScript)